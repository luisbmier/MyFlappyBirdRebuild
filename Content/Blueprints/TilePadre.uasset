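; TilePadre is a base level tile for a side-scroller that chains the spawning of the next tile.
; When the SideScrollerCharacter overlaps its next-tile trigger box, it asks the game mode to spawn the tile class set in Tile2Spawn.
; The game mode reference is cached in the construction script, and an IncrementPoints event adds to its score.
; Each tile destroys itself after a fixed delay from BeginPlay.
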(event OnComponentBeginOverlap(BoxNextTileTrigger)
  (params (OverlappedComponent :type Primitive%20Component%20Object%20Reference) (OtherActor :type Actor%20Object%20Reference) (OtherComp :type Primitive%20Component%20Object%20Reference) (OtherBodyIndex :type Integer) (bFromSweep :type Boolean) (SweepResult :type Hit%20Result%20Structure%20%28by%20ref%29))
  (Utilities|Casting|CastToSideScrollerCharacter OtherActor)
  (Default|SpawnTile (Variables|Default|GetGM) (Variables|Default|GetTile2Spawn)))

(event Custom|IncrementPoints
  (Math|Integer|IncrementInt (Variables|/Game/SideScrollerBP/Blueprints/SideScrollerGameMode.SideScrollerGameMode_C|Getpoints (Variables|Default|GetGM))))

(event Collision|EventActorBeginOverlap
  (params (OtherActor :type Actor%20Object%20Reference)))

(event EventTick
  (params (DeltaSeconds :type Float%20%28single-precision%29)))

(event EventBeginPlay
  (Utilities|FlowControl|Delay 9e+01)
  (Actor|DestroyActor))

(fn ConstructionScript
  (bind _asside_scroller_game_mode (Utilities|Casting|CastToSideScrollerGameMode (Game|GetGameMode)))
  (Variables|Default|SetGM _asside_scroller_game_mode))