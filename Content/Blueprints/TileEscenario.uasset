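; Scenery tile for a side-scroller that varies its backdrop at runtime and carries a box trigger that kills the player.
; On BeginPlay, helper functions give its hill, tree, mountain and MSnow mesh components a random mesh from per-category template arrays plus a random yaw.
; When the SideScrollerCharacter enters the Box, the tile calls PlayerDies on the SideScrollerGameMode.
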(event OnComponentBeginOverlap(Box)
  (params (OverlappedComponent :type Primitive%20Component%20Object%20Reference) (OtherActor :type Actor%20Object%20Reference) (OtherComp :type Primitive%20Component%20Object%20Reference) (OtherBodyIndex :type Integer) (bFromSweep :type Boolean) (SweepResult :type Hit%20Result%20Structure%20%28by%20ref%29))
  (Utilities|Casting|CastToSideScrollerCharacter OtherActor)
  (bind _asside_scroller_game_mode (Utilities|Casting|CastToSideScrollerGameMode (Game|GetGameMode)))
  (Default|PlayerDies _asside_scroller_game_mode))

(event EventBeginPlay
  (|CallParentFunction)
  (CallFunction|RandomizeStaticMesh (Variables|Default|GetCollina) (Variables|Default|GetcolinasTemplate))
  (CallFunction|RandomizeArray (Utilities|Array|MakeArray (Variables|Default|GetArbol) (Variables|Default|GetArbol2) (Variables|Default|GetArbol3) (Variables|Default|GetArbol4) (Variables|Default|Getarbol5) (Variables|Default|Getarbol6) (Variables|Default|Getarbol7) (Variables|Default|Getarbol8) (Variables|Default|Getarbol9)) (Variables|Default|GetarbolesTemplate))
  (CallFunction|RandomizeStaticMesh (Variables|Default|Getmount) (Variables|Default|GetmountainsTemplate))
  (CallFunction|RandomizeArray (Utilities|Array|MakeArray (Variables|Default|Getmount) (Variables|Default|GetStaticMesh5) (Variables|Default|GetStaticMesh6)) (Variables|Default|GetmountainsTemplate))
  (CallFunction|RandomizeArray (Utilities|Array|MakeArray (Variables|Default|GetStaticMesh7) (Variables|Default|GetStaticMesh8) (Variables|Default|GetStaticMesh9)) (Variables|Default|GetMSnowTemplate)))

(event Collision|EventActorBeginOverlap
  (params (OtherActor :type Actor%20Object%20Reference))
  (|CallParentFunction OtherActor) ; This node is disabled and will not be called.\nDrag off pins to build functionality.
)

(event EventTick
  (params (DeltaSeconds :type Float%20%28single-precision%29))
  (|CallParentFunction DeltaSeconds) ; This node is disabled and will not be called.\nDrag off pins to build functionality.
)

(fn ConstructionScript
  (|CallParentFunction))

(fn RandomizeStaticMesh
  (params (Target :type Static%20Mesh%20Component%20Object%20Reference) (Array :type Array%20of%20Static%20Mesh%20Object%20References))
  (bind _relativerotation (Variables|/Script/Engine.SceneComponent|GetRelativeRotation Target))
  (bind (_roll _pitch) (Math|Rotator|BreakRotator _relativerotation))
  (Components|StaticMesh|SetStaticMesh Target (Utilities|Array|Get(acopy) Array (Math|Random|RandomIntegerinRange 0 (- (Utilities|Array|Length Array) 1))))
  (Transformation|SetRelativeRotation Target (Math|Rotator|MakeRotator _roll _pitch (Math|Random|RandomFloatinRange 0.0 3.6e+02)) false false)
  (return))

(fn RandomizeArray
  (params (Array :type Array%20of%20Static%20Mesh%20Component%20Object%20References) (Array1 :type Array%20of%20Static%20Mesh%20Object%20References))
  (for _index (range 0 (- (Utilities|Array|Length Array) 1))
    (CallFunction|RandomizeStaticMesh (Utilities|Array|Get(acopy) Array _index) Array1)))