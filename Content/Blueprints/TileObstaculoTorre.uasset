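; Tower obstacle tile, a child Blueprint that varies the height of its obstacle and awards points on overlap.
; On BeginPlay it picks one random vertical offset and uses a macro to teleport the tower, child actor and next-tile trigger by that same amount along world Z.
; Actor overlap runs the parent handler, then calls IncrementPoints without checking which actor entered.
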(event EventBeginPlay
  (|CallParentFunction)
  (bind _output_get (Variables|Default|SetNewVar_0_0 (Math|Random|RandomFloatinRange -5e+01 3.5e+02)))
  (Utilities|NewMacro0 (Variables|Default|GetTorre) _output_get)
  (Utilities|NewMacro0 (Variables|Default|GetChildActor) _output_get)
  (Utilities|NewMacro0 (Variables|Default|GetBoxNextTileTrigger) _output_get))

(event Collision|EventActorBeginOverlap
  (params (OtherActor :type Actor%20Object%20Reference))
  (|CallParentFunction OtherActor)
  (CallFunction|IncrementPoints))

(event EventTick
  (params (DeltaSeconds :type Float%20%28single-precision%29))
  (|CallParentFunction DeltaSeconds) ; This node is disabled and will not be called.\nDrag off pins to build functionality.
)

(fn ConstructionScript
  (|CallParentFunction))